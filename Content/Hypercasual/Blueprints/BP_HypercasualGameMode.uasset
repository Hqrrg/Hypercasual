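; Game mode for the hypercasual boulder game that handles the start and end of each run.
; One tick after BeginPlay, it either shows the main menu and clears the game instance's ShouldDisplayMainMenu flag, or starts the boulder pawn's physics movement directly.
; EndGame extends the parent's logic by opening the end-game widget with the distance travelled and new-high-score values.
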(event `self.ReceiveBeginPlay`
  (`parent.ReceiveBeginPlay`)
  (`KismetSystemLibrary.DelayUntilNextTick`)
  (if (`HypercasualGameInstance.ShouldDisplayMainMenu` (`self.HypercasualGameInstance`))
    (bind _returnvalue (`|CreateWidget` "/Game/Hypercasual/Blueprints/UI/WBP_MainMenu.WBP_MainMenu_C" (`GameplayStatics.GetPlayerController` 0)))
    (`UserWidget.AddToViewport` _returnvalue 0)
    (set `HypercasualGameInstance.ShouldDisplayMainMenu` false (`self.HypercasualGameInstance`))
    (else
      (bind _asbp_boulder (cast `/Game/Hypercasual/Blueprints/BP_Boulder` (`GameplayStatics.GetPlayerPawn` 0)))
      (`Boulder.BeginPhysicsMovement` _asbp_boulder))))

(event `self.EndGame`
  (params (DistanceTravelled :type "Float (single-precision)") (NewHighScore :type Boolean))
  (`parent.EndGame` DistanceTravelled NewHighScore)
  (bind _returnvalue (`|CreateWidget` "/Game/Hypercasual/Blueprints/UI/WBP_EndGame.WBP_EndGame_C" (`GameplayStatics.GetPlayerController` 0) NewHighScore DistanceTravelled))
  (`UserWidget.AddToViewport` _returnvalue 0))

(fn `UserConstructionScript`)